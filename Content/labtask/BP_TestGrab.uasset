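; BP_TestGrab is a test actor with a Cube that can be gripped and dropped.
; On BeginPlay it binds handlers to the OnGrip and OnDrop events of its BPCGripStaticMesh component.
; Grip attaches the Cube to the supplied grab component with keep-relative rules.
; Drop turns on physics simulation and detaches the Cube.
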(event Custom|CustomEvent_0
  (params (GrabComp :type Primitive%20Component%20Object%20Reference)))

(event EventBeginPlay
  (bind _bpc_gripstaticmesh (Variables|Default|GetBPC_GripStaticMesh))
  (EventDispatchers|BindEventtoOnGrip _bpc_gripstaticmesh (EventDispatchers|CreateEvent :!event Grip))
  (EventDispatchers|BindEventtoOnDrop _bpc_gripstaticmesh (EventDispatchers|CreateEvent :!event Drop)))

(event Collision|EventActorBeginOverlap
  (params (OtherActor :type Actor%20Object%20Reference)))

(event EventTick
  (params (DeltaSeconds :type Float%20%28single-precision%29)))

(event EventGrip
  (params (GrabComp :type Primitive%20Component%20Object%20Reference))
  (Transformation|AttachComponentToComponent (Variables|Default|GetCube) GrabComp "None" "KeepRelative" "KeepRelative" "KeepRelative" true))

(event EventDrop
  (Physics|SetSimulatePhysics (Variables|Default|GetCube) true)
  (Transformation|DetachFromComponent (Variables|Default|GetCube) "KeepRelative" "KeepRelative" "KeepRelative" true))

(fn ConstructionScript)